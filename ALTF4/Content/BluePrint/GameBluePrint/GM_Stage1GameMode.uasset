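; Stage 1 game mode that handles player respawning and a single-use save sign checkpoint.
; BeginPlay records the PlayerStart location as the default and current spawn point.
; SaveSign_SpawnPoint moves the current point and spawns an active sign there, replacing any previous one.
; After a delay, Respawn spawns, possesses and initializes a new BP_Player; using a sign plays a break sound, destroys it and restores the default point.
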(event Custom|Respawn
  (params (inPlayerController :type Controller%20Object%20Reference))
  (Variables|Default|SetIn%20Player%20Controller inPlayerController)
  (Utilities|FlowControl|Delay 5.0)
  (if (Class|KismetMathLibrary|EqualExactlyVectorVector (Variables|Default|GetCurrentSpawnPoint) (Variables|Default|GetDefaultSpawnPoint))
    (Utilities|CurrentPositionSpawn)
    (else
      (Variables|Default|SetbSaveSignUsed false)
      (Audio|PlaySound2D "/Game/Sound/SFX/Item/Savesign_Borken_Sound.Savesign_Borken_Sound" 1.0 1.0 0.0 0 0)
      (Utilities|CurrentPositionSpawn)
      (Variables|Default|SetCurrentSpawnPoint (Variables|Default|GetDefaultSpawnPoint))
      (Actor|DestroyActor (Variables|Default|GetActiveSaveSign)))))

(event Custom|SaveSign_SpawnPoint
  (params (inSpawnPoint :type Vector))
  (Variables|Default|SetCurrentSpawnPoint inSpawnPoint)
  (if (Variables|Default|GetbSaveSignUsed)
    (Actor|DestroyActor (Variables|Default|GetActiveSaveSign))
    (Utilities|SpawnSaveSign)
    (else
      (Variables|Default|SetbSaveSignUsed true)
      (Utilities|SpawnSaveSign))))

(event EventBeginPlay
  (bind _returnvalue (Actor|GetActorOfClass "/Script/Engine.PlayerStart"))
  (Variables|Default|SetDefaultSpawnPoint (Transformation|GetActorLocation _returnvalue))
  (Variables|Default|SetCurrentSpawnPoint (Variables|Default|GetDefaultSpawnPoint)))

(fn ConstructionScript)