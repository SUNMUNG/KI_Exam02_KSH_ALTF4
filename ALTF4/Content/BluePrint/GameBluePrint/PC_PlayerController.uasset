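; Player controller that sets up input, the HUD and the pause menu for the local player.
; On BeginPlay it adds the Enhanced Input mapping context, shows the character HUD and loads settings through BP_GameInstance.
; Escape or P toggles pause: pausing creates the pause menu widget and shows the cursor, while resuming removes it, hides the cursor and restores game-only input.
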(event Custom|ResumeGame
  (bind _settingmenuwidget (Variables|Default|GetSettingMenuWidget))
  (Game|SetGamePaused false)
  (Variables|Default|SetbShowMouseCursor false)
  (Input|SetInputModeGameOnly self false)
  (Utilities|IsValid _settingmenuwidget
    (:Is%20Valid
      (Widget|RemovefromParent _settingmenuwidget))))

(event Custom|PauseGame
  (Game|SetGamePaused true)
  (bind _returnvalue (UserInterface|CreateWidget "/Game/UI/WBP_PauseMenu.WBP_PauseMenu_C"))
  (bind _output_get (Variables|Default|SetSettingMenuWidget _returnvalue))
  (UserInterface|Viewport|AddtoViewport _output_get 0)
  (Variables|Default|SetbShowMouseCursor true))

(event EventBeginPlay
  (Input|AddMappingContext (PlayerController|LocalPlayerSubsystems|GetEnhancedInputLocalPlayerSubsystem) "/Game/Input/IMC_Control.IMC_Control" 0 "(bIgnoreAllPressedKeysUntilRelease=True,bForceImmediately=False,bNotifyUserSettings=False)")
  (bind _returnvalue (UserInterface|CreateWidget "/Game/UI/WP_CharacterHud.WP_CharacterHud_C" self))
  (bind _output_get (Variables|Default|SetHUDWidget _returnvalue))
  (UserInterface|Viewport|AddtoViewport _output_get 0)
  (bind _asbp_game_instance (Utilities|Casting|CastToBP_GameInstance (Game|GetGameInstance)))
  (Default|LoadSettings _asbp_game_instance))

(event Input|KeyboardEvents|Escape
  (params (Key :type Key%20Structure :default "None"))
  ;[0.15 0.15 0.15 0.5] ESC or P 누르면 게임중지
  (:Pressed
    (if (Game|IsGamePaused)
      (CallFunction|ResumeGame)
      (else
        (CallFunction|PauseGame)))))

(event Input|KeyboardEvents|P
  (params (Key :type Key%20Structure :default "None"))
  ;[0.15 0.15 0.15 0.5] ESC or P 누르면 게임중지
  (:Pressed
    (if (Game|IsGamePaused)
      (CallFunction|ResumeGame)
      (else
        (CallFunction|PauseGame)))))

(fn ConstructionScript)