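; BP_Player is the player character, with camera-relative movement, sprint, jump, right-click aim zoom via timeline and montage-driven chicken throwing on a cooldown.
; Hits on tagged components either launch it or cost a heart and trigger ragdoll.
; A looping timer ends ragdoll once velocity settles, then a pelvis dot product picks the front or back get-up montage.
; Death, drowning or suicide input shows death UI and respawns through the game mode.
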(event Custom|RagdollState
  ;[0.15 0.15 0.15 0.5] Ragdoll 상태 만들기
  (Variables|Default|SetbisRagdoll true)
  (Utilities|LieDownActivate)
  (Utilities|Time|SetTimerbyFunctionName 0 "CheckRagdollStability" 0.1 true))

(event Custom|ThrowChicken
  ;[0.15 0.15 0.15 0.5] 닭 발사
  (if (Variables|Default|GetbCanFire)
    (Game|SpawnActorfromClass "/Game/BluePrint/Player/BP_ThrowChicken.BP_ThrowChicken_C" (Math|Transform|MakeTransform (Transformation|GetWorldLocation (Variables|Default|GetThrowPoint)) "0, 0, 0" "0.500000,0.500000,0.500000") "AdjustIfPossibleButDontSpawnIfColliding" "MultiplyWithRoot" 0 0)
    (Variables|Default|SetbCanFire false)))

(event Custom|InWaterDead
  ;[0.15 0.15 0.15 0.5] 사망처리
  (Audio|PlaySound2D "/Game/Sound/SFX/TrapSound/물에빠지는효과음_Fix.물에빠지는효과음_Fix" 1.0 1.0 0.0 0 0)
  (Audio|PlaySound2D "/Game/Sound/SFX/Character/voice_male_b_death_high_04.voice_male_b_death_high_04" 1.0 1.0 0.0 0 0)
  (Game|SpawnActorfromClass "/Game/BluePrint/Player/BP_DeadBody.BP_DeadBody_C" (Math|Transform|MakeTransform (Transformation|GetWorldLocation (Variables|Character|GetMesh)) "0, 0, 0" "1.000000,1.000000,1.000000") "Undefined" "MultiplyWithRoot" 0 0)
  (Default|YouDiedVisible (Variables|Default|GetHUDWidget))
  (Utilities|RespawnMacro))

(event Custom|StartManualTurn
  (params (inTurn :type Float%20%28double-precision%29))
  ;[0.15 0.15 0.15 0.5] 제자리 회전 커스텀 이벤트
  (bind _output_get (Variables|Default|SetTurnStartRotation (Transformation|GetActorRotation)))
  (bind _alpha (Timeline|TL_Turn PlayFromStart)
    (:Update
      (Transformation|SetActorRotation (Math|Rotator|Lerp(Rotator) (Variables|Default|GetTurnStartRotation) (Math|Rotator|MakeRotator (.roll _output_get) (.pitch _output_get) (+ (.yaw _output_get) inTurn)) _alpha)))))

(event Custom|CharacterInitialize
  ;[0.15 0.15 0.15 0.5] 플레이어 체력 초기화 UI연동
  (Variables|Default|SetPlayerHealth (Variables|Default|GetDefaultPlayerHealth))
  (bind _aspc_player_controller (Utilities|Casting|CastToPC_PlayerController (Pawn|GetController)))
  (bind _output_get (Variables|Default|SetWP%20Health (Variables|/Game/UI/WP_CharacterHud.WP_CharacterHud_C|GetWP_Health (Variables|/Game/BluePrint/GameBluePrint/PC_PlayerController.PC_PlayerController_C|GetHUDWidget _aspc_player_controller))))
  (Default|UpdateHearts _output_get (Variables|Default|GetPlayerHealth)))

(event Custom|GetUpAnim
  ;[0.15 0.15 0.15 0.5] 일어나는 애니메이션
  (bind _returnvalue (CallFunction|GetUpState))
  (if _returnvalue
    (Animation|Montage|PlayMontage (Variables|Character|GetMesh) "/Game/Animation/Character/AM_GetUpFront.AM_GetUpFront"
      (:OnCompleted
        _))
    (else
      (Animation|Montage|PlayMontage (Variables|Character|GetMesh) "/Game/Animation/Character/AM_GetUpBack.AM_GetUpBack"
        (:OnCompleted
          _))))
  (Pawn|Components|CharacterMovement|SetMovementMode (Variables|Character|GetCharacterMovement) "MOVE_Walking" 0)
  (Variables|Default|SetbisRagdoll false))

(event Custom|NormalView
  (bind _springarm (Variables|Default|GetSpringArm))
  (Variables|/Script/Engine.CharacterMovementComponent|SetbOrientRotationToMovement (Variables|Character|GetCharacterMovement) true)
  (Variables|/Script/Engine.SpringArmComponent|SetbUsePawnControlRotation (Variables|Default|GetSpringArm) true)
  (Variables|Default|SetbUseControllerRotationYaw false)
  (Default|AimVisibleChange (Variables|Default|GetHUDWidget))
  (bind _alpha (Timeline|TL_AimVIew Reverse)
    (:Update
      (Variables|/Script/Engine.SpringArmComponent|SetTargetArmLength _springarm (Math|Float|Lerp (Variables|Default|GetNormalView_ArmLength) (Variables|Default|GetAimView_ArmLength) _alpha))
      (Variables|/Script/Engine.SpringArmComponent|SetTargetOffset _springarm (Math|Vector|Lerp(Vector) "0.000000,0.000000,150.000000" "0.000000,0.000000,200.000000" _alpha)))))

(event Custom|AimViewChange
  (bind _springarm (Variables|Default|GetSpringArm))
  (Variables|/Script/Engine.CharacterMovementComponent|SetbOrientRotationToMovement (Variables|Character|GetCharacterMovement) false)
  (Variables|Default|SetbUseControllerRotationYaw true)
  (bind _alpha (Timeline|TL_AimVIew Play)
    (:Update
      (Variables|/Script/Engine.SpringArmComponent|SetTargetArmLength _springarm (Math|Float|Lerp (Variables|Default|GetNormalView_ArmLength) (Variables|Default|GetAimView_ArmLength) _alpha))
      (Variables|/Script/Engine.SpringArmComponent|SetTargetOffset _springarm (Math|Vector|Lerp(Vector) "0.000000,0.000000,150.000000" "0.000000,0.000000,200.000000" _alpha)))))

(event Input|EnhancedActionEvents|EnhancedInputActionIA_Move
  (params (ActionValue :type Vector%202D%20Structure) (ElapsedSeconds :type Float%20%28double-precision%29) (TriggeredSeconds :type Float%20%28double-precision%29) (InputAction :type Input%20Action%20Object%20Reference :default "/Game/Input/IA_Move.IA_Move"))
  ;[0.15 0.15 0.15 0.5] 자유시점 카메라에 맞춘 이동
  (:Triggered
    (Variables|Default|SetYMove (.y ActionValue))
    (Variables|Default|SetXMove (.x ActionValue))
    (Pawn|Input|AddMovementInput (Utilities|MoveDirection (.x ActionValue) (.y ActionValue)) 1.0 false))
  (:Completed
    (Variables|Default|SetYMove 0.0)
    (Variables|Default|SetXMove 0.0)))

(event Input|EnhancedActionEvents|EnhancedInputActionIA_CameraMove
  (params (ActionValue :type Vector%202D%20Structure) (ElapsedSeconds :type Float%20%28double-precision%29) (TriggeredSeconds :type Float%20%28double-precision%29) (InputAction :type Input%20Action%20Object%20Reference :default "/Game/Input/IA_CameraMove.IA_CameraMove"))
  ;[0.15 0.15 0.15 0.5] 카메라 이동 ( 폰 제어 회전 가능 true)
  (Pawn|Input|AddControllerPitchInput (* (.y ActionValue) -1.0))
  (Pawn|Input|AddControllerYawInput (.x ActionValue)))

(event Input|EnhancedActionEvents|EnhancedInputActionIA_Sprint
  (params (ActionValue :type Boolean) (ElapsedSeconds :type Float%20%28double-precision%29) (TriggeredSeconds :type Float%20%28double-precision%29) (InputAction :type Input%20Action%20Object%20Reference :default "/Game/Input/IA_Sprint.IA_Sprint"))
  ;[0.15 0.15 0.15 0.5] Sprint 세팅
  (:Triggered
    (Variables|/Script/Engine.CharacterMovementComponent|SetMaxWalkSpeed (Variables|Character|GetCharacterMovement) (Variables|Default|GetSprintSpeed)))
  (:Canceled
    (Variables|/Script/Engine.CharacterMovementComponent|SetMaxWalkSpeed (Variables|Character|GetCharacterMovement) (Variables|Default|GetMoveSpeed) :!label _label))
  (:Completed
    (goto _label)))

(event Input|EnhancedActionEvents|EnhancedInputActionIA_Jump
  (params (ActionValue :type Boolean) (ElapsedSeconds :type Float%20%28double-precision%29) (TriggeredSeconds :type Float%20%28double-precision%29) (InputAction :type Input%20Action%20Object%20Reference :default "/Game/Input/IA_Jump.IA_Jump"))
  ;[0.15 0.15 0.15 0.5] 점프
  (:Triggered
    (Character|Jump))
  (:Completed
    (Character|StopJumping)))

(event Input|EnhancedActionEvents|EnhancedInputActionIA_LieDown
  (params (ActionValue :type Boolean) (ElapsedSeconds :type Float%20%28double-precision%29) (TriggeredSeconds :type Float%20%28double-precision%29) (InputAction :type Input%20Action%20Object%20Reference :default "/Game/Input/IA_LieDown.IA_LieDown"))
  ;[0.15 0.15 0.15 0.5] Ragdoll 상태 만들기
  (:Started
    (if (not (Variables|Default|GetbisRagdoll))
      (CallFunction|RagdollState))))

(event Input|EnhancedActionEvents|EnhancedInputActionIA_ViewChange
  (params (ActionValue :type Boolean) (ElapsedSeconds :type Float%20%28double-precision%29) (TriggeredSeconds :type Float%20%28double-precision%29) (InputAction :type Input%20Action%20Object%20Reference :default "/Game/Input/IA_ViewChange.IA_ViewChange"))
  ;[0.15 0.15 0.15 0.5] 우클릭시 arm length 조절 (줌인)
  (:Triggered
    (CallFunction|AimViewChange))
  (:Started
    (Default|AimVisibleChange (Variables|Default|GetHUDWidget)))
  (:Completed
    (CallFunction|NormalView)))

(event Input|EnhancedActionEvents|EnhancedInputActionIA_Throw
  (params (ActionValue :type Boolean) (ElapsedSeconds :type Float%20%28double-precision%29) (TriggeredSeconds :type Float%20%28double-precision%29) (InputAction :type Input%20Action%20Object%20Reference :default "/Game/Input/IA_Throw.IA_Throw"))
  ;[0.15 0.15 0.15 0.5] 닭 던지기 애니메이션 재생 (노티파이로 닭생성)
  (:Started
    (if (and (Variables|Default|GetbCanFire) (not (Variables|Default|GetbisRagdoll)))
      (Animation|PlayAnimMontage "/Game/Animation/Character/AM_ThrowChicken.AM_ThrowChicken" 1.0 "None")
      (Utilities|FlowControl|Delay 2.0)
      (Variables|Default|SetbCanFire true))))

(event Input|EnhancedActionEvents|EnhancedInputActionIA_Suicide
  (params (ActionValue :type Boolean) (ElapsedSeconds :type Float%20%28double-precision%29) (TriggeredSeconds :type Float%20%28double-precision%29) (InputAction :type Input%20Action%20Object%20Reference :default "/Game/Input/IA_Suicide.IA_Suicide"))
  ;[0.15 0.15 0.15 0.5] G 누르면 리스폰
  (:Started
    (Utilities|DieProcess)))

(event EventTick
  (params (DeltaSeconds :type Float%20%28single-precision%29))
  ;[0.15 0.15 0.15 0.5] 점프중인지 체크 (틱 안쓰는 법 있으면 수정예정)
  (Variables|Default|SetisFlying (AI|Components|NavMovement|IsFalling (Variables|Character|GetCharacterMovement))))

(event Collision|EventHit
  (params (MyComp :type Primitive%20Component%20Object%20Reference) (Other :type Actor%20Object%20Reference) (OtherComp :type Primitive%20Component%20Object%20Reference) (bSelfMoved :type Boolean) (HitLocation :type Vector :default "0, 0, 0") (HitNormal :type Vector :default "0, 0, 0") (NormalImpulse :type Vector :default "0, 0, 0") (Hit :type Hit%20Result%20Structure%20%28by%20ref%29))
  (bind _returnvalue (* (.impactnormal Hit) 1e+03))
  ;[0.15 0.15 0.15 0.5] Ragdolable 태그면 래그돌 상태후 indamaged  LaunchAble태그면 발사
  (Variables|Default|SetOther%20Comp OtherComp)
  (Utilities|FlowControl|Sequence
    (:then_0
      (if (Components|ComponentHasTag (Variables|Default|GetOther%20Comp) "Ragdollable")
        (CallFunction|RagdollState)
        (Audio|PlaySound2D "/Game/Sound/SFX/Character/voice_male_b_hurt_pain_set_1_01.voice_male_b_hurt_pain_set_1_01" 1.0 1.0 0.0 0 0)
        (Utilities|InDamaged
          (:Execute1
            (if (<= (Variables|Default|GetPlayerHealth) 0)
              (Audio|PlaySound2D "/Game/Sound/SFX/Character/voice_male_b_death_high_06.voice_male_b_death_high_06" 1.0 1.0 0.0 0 0)
              (Utilities|DieProcess))))))
    (:then_1
      (if (Components|ComponentHasTag (Variables|Default|GetOther%20Comp) "LaunchAble")
        (Character|LaunchCharacter (Math|Vector|MakeVector (.x _returnvalue) (.y _returnvalue) 1e+03) true false)))))

(event EventBeginPlay
  ;[0.15 0.15 0.15 0.5] beginplay 에서 초기값 설정
  (Utilities|FlowControl|Delay 0.5)
  (Utilities|IsValid (Variables|Default|GetHUDWidget)
    (:Is%20Valid
      (CallFunction|CharacterInitialize))
    (:Is%20Not%20Valid
      (bind _aspc_player_controller (Utilities|Casting|CastToPC_PlayerController (Pawn|GetController)))
      (Variables|Default|SetHUDWidget (Variables|/Game/BluePrint/GameBluePrint/PC_PlayerController.PC_PlayerController_C|GetHUDWidget _aspc_player_controller))
      (CallFunction|CharacterInitialize))))

(fn ConstructionScript)

(fn CheckRagdollStability
  ;[0.15 0.15 0.15 0.5] 상태 안정화되면 래그돌 해제
  (bind _returnvalue (Physics|GetPhysicsLinearVelocity (Variables|Character|GetMesh) "None"))
  (if (<= (Math|Vector|VectorLength _returnvalue) 5.0)
    (Utilities|Time|ClearTimerbyFunctionName 0 "CheckRagdollStability")
    (Utilities|LieDownDeActivate)))

(fn GetUpState
  (return (> (Math|Vector|DotProduct (Math|Vector|GetRightVector (Transformation|GetSocketRotation (Variables|Character|GetMesh) "pelvis")) (Math|Vector|VectorUp)) 0.0)))