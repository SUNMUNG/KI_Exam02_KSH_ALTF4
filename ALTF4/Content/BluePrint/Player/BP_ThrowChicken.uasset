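; BP_ThrowChicken is a thrown chicken projectile that turns into a ragdoll when it hits something.
; On BeginPlay it sets its ProjectileMovement velocity along the BP_Player camera's forward vector, scaled by ChickenImpulsePower, with a fixed upward boost for an arc.
; On hit it disables capsule collision, switches the skeletal mesh to ragdoll physics, and destroys itself after a delay.
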(event EventBeginPlay
  (bind _asbp_player (Utilities|Casting|CastToBP_Player (Game|Player|GetPlayerPawn 0)))
  (Variables|/Script/Engine.MovementComponent|SetVelocity (Variables|Default|GetProjectileMovement) (+ (* (Math|Vector|GetForwardVector (Variables|/Game/BluePrint/Player/BP_Player.BP_Player_C|GetCamera _asbp_player)) (Variables|Default|GetChickenImpulsePower)) "0.000000,0.000000,500.000000")))

(event Collision|EventHit
  (params (MyComp :type Primitive%20Component%20Object%20Reference) (Other :type Actor%20Object%20Reference) (OtherComp :type Primitive%20Component%20Object%20Reference) (bSelfMoved :type Boolean) (HitLocation :type Vector :default "0, 0, 0") (HitNormal :type Vector :default "0, 0, 0") (NormalImpulse :type Vector :default "0, 0, 0") (Hit :type Hit%20Result%20Structure%20%28by%20ref%29))
  (bind _skeletalmesh (Variables|Default|GetSkeletalMesh))
  (Collision|SetCollisionProfileName (Variables|Default|GetCapsule) "NoCollision" true :!class /Script/Engine.PrimitiveComponent)
  (Physics|SetSimulatePhysics _skeletalmesh true)
  (Collision|SetCollisionProfileName _skeletalmesh "Ragdoll" true :!class /Script/Engine.PrimitiveComponent)
  (Utilities|FlowControl|Delay 1e+01)
  (Actor|DestroyActor))

(fn ConstructionScript)