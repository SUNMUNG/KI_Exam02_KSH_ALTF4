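; BP_Player is the player Blueprint, handling Enhanced Input for camera look, movement, jumping and throwing.
; Camera input drives controller pitch and yaw, and movement always pushes along the control yaw's forward vector, ignoring the input value.
; Throwing spawns a half-scale BP_ThrowChicken at ThrowPoint and applies a fixed world +X impulse to its sphere, independent of aim.
; An unconnected MoveSpeed-based movement node never runs.
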(event Input|EnhancedActionEvents|EnhancedInputActionIA_Move
  (params (ActionValue :type Vector%202D%20Structure) (ElapsedSeconds :type Float%20%28double-precision%29) (TriggeredSeconds :type Float%20%28double-precision%29) (InputAction :type Input%20Action%20Object%20Reference :default "/Game/Input/IA_Move.IA_Move"))
  ;[0.15 0.15 0.15 0.5] 카메라로 바라보고 있는 방향으로 이동
  (Pawn|Input|AddMovementInput (Math|Vector|GetForwardVector (Math|Rotator|MakeRotator 0.0 0.0 (.yaw (Pawn|GetControlRotation :!class /Script/Engine.Pawn)))) 1.0 false))

(event Input|EnhancedActionEvents|EnhancedInputActionIA_CameraMove
  (params (ActionValue :type Vector%202D%20Structure) (ElapsedSeconds :type Float%20%28double-precision%29) (TriggeredSeconds :type Float%20%28double-precision%29) (InputAction :type Input%20Action%20Object%20Reference :default "/Game/Input/IA_CameraMove.IA_CameraMove"))
  ;[0.15 0.15 0.15 0.5] 카메라 이동 ( 폰 제어 회전 가능 true)
  (Pawn|Input|AddControllerPitchInput (.y ActionValue))
  (Pawn|Input|AddControllerYawInput (.x ActionValue)))

(event Input|EnhancedActionEvents|EnhancedInputActionIA_Throw
  (params (ActionValue :type Boolean) (ElapsedSeconds :type Float%20%28double-precision%29) (TriggeredSeconds :type Float%20%28double-precision%29) (InputAction :type Input%20Action%20Object%20Reference :default "/Game/Input/IA_Throw.IA_Throw"))
  (:Started
    (bind _returnvalue (Game|SpawnActorfromClass "/Game/BluePrint/BP_ThrowChicken.BP_ThrowChicken_C" (Math|Transform|MakeTransform (Transformation|GetWorldLocation (Variables|Default|GetThrowPoint)) "0, 0, 0" "0.500000,0.500000,0.500000") "Undefined" "MultiplyWithRoot" 0 0))
    (Physics|AddImpulse (Variables|/Game/BluePrint/BP_ThrowChicken.BP_ThrowChicken_C|GetSphere _returnvalue) "10000.000000,0.000000,0.000000" "None" false)))

(event Input|EnhancedActionEvents|EnhancedInputActionIA_Jump
  (params (ActionValue :type Boolean) (ElapsedSeconds :type Float%20%28double-precision%29) (TriggeredSeconds :type Float%20%28double-precision%29) (InputAction :type Input%20Action%20Object%20Reference :default "/Game/Input/IA_Jump.IA_Jump"))
  ;[0.15 0.15 0.15 0.5] 점프
  (Character|Jump))

(fn ConstructionScript)