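; BP_Guilotine is a guillotine trap whose blade moves vertically between a maximum and minimum height.
; On BeginPlay it waits an initial delay, then starts the TL_BladeMove timeline, which lerps the Blade's relative location without sweeping.
; An exact check for an alpha of 1.0 in the timeline update plays a sound at the actor's location when the blade reaches minimum height.
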(event EventBeginPlay
  (Utilities|FlowControl|Delay (Variables|Default|GetInitialDelay))
  (bind _blademove (Timeline|TL_BladeMove PlayFromStart)
    (:Update
      (Transformation|SetRelativeLocation (Variables|Default|GetBlade) (Math|Vector|Lerp(Vector) (Math|Vector|MakeVector 0.0 0.0 (Variables|Default|GetMaxHeight)) (Math|Vector|MakeVector 0.0 0.0 (Variables|Default|GetMinHeight)) _blademove) false false)
      (if (== _blademove 1.0)
        (Audio|PlaySoundatLocation "/Game/Sound/SFX/TrapSound/11_전기톱날2.11_전기톱날2" (Transformation|GetActorLocation) "0, 0, 0" 1.0 1.0 0.0 0 0 0 0)))))

(fn ConstructionScript)