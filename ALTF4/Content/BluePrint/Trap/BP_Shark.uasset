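; BP_Shark is a trap actor that launches a physics box along a ballistic arc when play begins.
; It solves a toss velocity toward a point offset along the box's right vector by TargetLocation, with debug drawing enabled.
; If a solution exists, the velocity is applied as a mass-independent impulse and the actor gets a limited lifespan; otherwise nothing happens.
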(event EventBeginPlay
  (bind _box (Variables|Default|GetBox))
  (bind _returnvalue (Transformation|GetWorldLocation _box))
  (bind (_tossvelocity _returnvalue_2) (Class|GameplayStatics|BlueprintSuggestProjectileVelocity _returnvalue (+ _returnvalue (* (Math|Vector|GetRightVector _box) (Variables|Default|GetTargetLocation))) 2e+03 0.0 "DoNotTrace" 0.0 false true false))
  (if _returnvalue_2
    (Physics|AddImpulse (Variables|Default|GetBox) _tossvelocity "None" true)
    (Actor|SetLifeSpan 1e+01)))

(fn ConstructionScript)