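; BP_ArrowTrap2 is a trap that repeatedly fires arrows on a timer.
; One second after BeginPlay, it starts a looping timer whose interval comes from a spawn-time variable.
; Each tick of the timer spawns a BP_Arrow at the ArrowPoint location with the trap's rotation.
; The arrow is launched by a physics impulse along ArrowPoint's horizontal forward direction, with a fixed upward component for lift.
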(event Custom|ArrowAttack
  (bind _arrowpoint (Variables|Default|GetArrowPoint))
  (bind _returnvalue (Math|Vector|GetForwardVector _arrowpoint))
  (bind _returnvalue_2 (Game|SpawnActorfromClass "/Game/BluePrint/Trap/BP_Arrow.BP_Arrow_C" (Math|Transform|MakeTransform (Transformation|GetWorldLocation (Variables|Default|GetArrowPoint)) (Transformation|GetActorRotation) "1.000000,1.000000,1.000000") "Undefined" "MultiplyWithRoot" 0 0))
  (Physics|AddImpulse (Variables|/Game/BluePrint/Trap/BP_Arrow.BP_Arrow_C|GetArrow _returnvalue_2) (Math|Vector|MakeVector (* (.x _returnvalue) 1.5e+04) (* (.y _returnvalue) 1.5e+04) 1e+03) "None" false))

(event EventBeginPlay
  (Utilities|FlowControl|Delay 1.0)
  (Utilities|Time|SetTimerbyEvent (delegate Custom|ArrowAttack) (Variables|Default|GetAroorwSpawnTime) true))

(fn ConstructionScript)