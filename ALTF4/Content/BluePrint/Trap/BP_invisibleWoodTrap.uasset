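; Invisible wooden trap that appears with a sound and swings out when an actor overlaps it, knocking back the player on hit.
; Timed RotatingMovement rate changes swing it quickly, then return it at half speed after overlap ends, with IsPending blocking retriggers until reset.
; A hit from the player pawn launches BP_Player along a fixed backward-and-up world vector.
; Once revealed, the trap stays visible.
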(event Collision|EventActorBeginOverlap
  (params (OtherActor :type Actor%20Object%20Reference))
  (bind _rotatingmovement (Variables|Default|GetRotatingMovement))
  ;[0.15 0.15 0.15 0.5] 회전 컴포넌트 사용
  (if (not (Variables|Default|GetisPending))
    (Audio|PlaySound2D "/Game/Sound/SFX/TrapSound/방방.방방" 1.0 1.0 0.0 0 0)
    (Variables|Default|SetisPending true)
    (Rendering|SetVisibility (Variables|Default|GetRoot) true true)
    (Variables|/Script/Engine.RotatingMovementComponent|SetRotationRate _rotatingmovement "200.000000,0.000000,0.000000")
    (Utilities|FlowControl|Delay 0.3)
    (Variables|/Script/Engine.RotatingMovementComponent|SetRotationRate _rotatingmovement "0, 0, 0")))

(event EventBeginPlay
  (Rendering|SetVisibility (Variables|Default|GetRoot) false true))

(event Collision|EventActorEndOverlap
  (params (OtherActor :type Actor%20Object%20Reference))
  (bind _rotatingmovement (Variables|Default|GetRotatingMovement))
  ;[0.15 0.15 0.15 0.5] 회전 컴포넌트 사용
  (if (Variables|Default|GetisPending)
    (Utilities|FlowControl|Delay 1.0)
    (Variables|/Script/Engine.RotatingMovementComponent|SetRotationRate _rotatingmovement "-100.000000,0.000000,0.000000")
    (Utilities|FlowControl|Delay 0.6)
    (Variables|/Script/Engine.RotatingMovementComponent|SetRotationRate _rotatingmovement "0, 0, 0")
    (Variables|Default|SetisPending false)))

(event Collision|EventHit
  (params (MyComp :type Primitive%20Component%20Object%20Reference) (Other :type Actor%20Object%20Reference) (OtherComp :type Primitive%20Component%20Object%20Reference) (bSelfMoved :type Boolean) (HitLocation :type Vector :default "0, 0, 0") (HitNormal :type Vector :default "0, 0, 0") (NormalImpulse :type Vector :default "0, 0, 0") (Hit :type Hit%20Result%20Structure%20%28by%20ref%29))
  (bind _returnvalue (Game|Player|GetPlayerPawn 0))
  (if (== _returnvalue Other)
    (bind _asbp_player (Utilities|Casting|CastToBP_Player _returnvalue))
    (Character|LaunchCharacter _asbp_player "-1500.000000,0.000000,1000.000000" true false)))

(fn ConstructionScript)