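; BP_SaveBalloon is a floating balloon item that spawns a BP_SaveSign when hit.
; On BeginPlay it sets its lifespan and plays a spawn sound, then nudges the Balloon component upward every Tick while Ishit is false, without delta-time scaling.
; Hit plays deflate and pop sounds, spawns the sign at the SaveSign component's location with a fixed rotation, and destroys the balloon.
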(event Custom|UpBallon
  (bind _balloon (Variables|Default|GetBalloon))
  (Transformation|SetRelativeLocation _balloon (+ (Variables|/Script/Engine.SceneComponent|GetRelativeLocation _balloon) "0.000000,0.000000,0.500000") false false))

(event EventBeginPlay
  (Actor|SetLifeSpan (Variables|Default|GetBalloonLifespan))
  (Audio|PlaySound2D "/Game/Sound/SFX/Item/4_풍선생성될때_효과음.4_풍선생성될때_효과음" 1.0 1.0 0.0 0 0))

(event EventTick
  (params (DeltaSeconds :type Float%20%28single-precision%29))
  (if (not (Variables|Default|Getishit))
    (CallFunction|UpBallon)))

(event Collision|EventHit
  (params (MyComp :type Primitive%20Component%20Object%20Reference) (Other :type Actor%20Object%20Reference) (OtherComp :type Primitive%20Component%20Object%20Reference) (bSelfMoved :type Boolean) (HitLocation :type Vector :default "0, 0, 0") (HitNormal :type Vector :default "0, 0, 0") (NormalImpulse :type Vector :default "0, 0, 0") (Hit :type Hit%20Result%20Structure%20%28by%20ref%29))
  (if true
    (Audio|PlaySound2D "/Game/Sound/SFX/Item/BalloonDeflate.BalloonDeflate" 1.0 1.0 0.0 0 0)
    (Game|SpawnActorfromClass "/Game/BluePrint/Item/BP_SaveSign.BP_SaveSign_C" (Math|Transform|MakeTransform (Transformation|GetWorldLocation (Variables|Default|GetSaveSign)) "0.000000,180.000000,0.000000" "1.000000,1.000000,1.000000") "Undefined" "MultiplyWithRoot" 0 0)
    (Audio|PlaySound2D "/Game/Sound/SFX/TrapSound/BalloonBoomSound.BalloonBoomSound" 1.0 1.0 0.0 0 0)
    (Actor|DestroyActor)))

(fn ConstructionScript)