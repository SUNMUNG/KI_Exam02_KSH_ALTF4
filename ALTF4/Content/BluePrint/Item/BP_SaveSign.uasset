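; BP_SaveSign is a one-shot checkpoint sign that sets the player's spawn point in Stage 1.
; When the player pawn overlaps it, it plays a 2D sound and casts the game mode to GM_Stage1GameMode.
; It passes the sign's world location, raised slightly, to SaveSignSpawnPoint, then destroys itself.
; If the cast fails, the sound still plays but the sign remains.
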(event Collision|EventActorBeginOverlap
  (params (OtherActor :type Actor%20Object%20Reference))
  (if (== (Game|Player|GetPlayerPawn 0) OtherActor)
    (Audio|PlaySound2D "/Game/Sound/SFX/Item/SaveSign_SpawnSound.SaveSign_SpawnSound" 1.0 1.0 0.0 0 0)
    (bind _asgm_stage_1game_mode (Utilities|Casting|CastToGM_Stage1GameMode (Game|GetGameMode)))
    (Default|SaveSignSpawnPoint _asgm_stage_1game_mode (+ (Transformation|GetWorldLocation (Variables|Default|GetSaveSign)) "0.000000,0.000000,50.000000"))
    (Actor|DestroyActor)))

(fn ConstructionScript)